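; BP_Bench is a bench actor that registers itself as a ride and spins continuously.
; On BeginPlay it passes the world transforms of two numbered "pos_" mesh sockets to the bench subsystem as socket locations, then adds itself as a ride.
; Tick adds a fixed rotation increment every frame without delta-time scaling, and the registered transforms are not updated afterwards.
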(event `self.ReceiveBeginPlay`
  (bind _returnvalue (subsystem `BenchSubsystem`))
  (bind _newparam (`self.GetSocketTransform` 0))
  (`BenchSubsystem.AddSocketLocation` _returnvalue _newparam)
  (bind _newparam_2 (`self.GetSocketTransform` 1))
  (`BenchSubsystem.AddSocketLocation` _returnvalue _newparam_2)
  (`BenchSubsystem.AddRide` _returnvalue self))

(event `self.ReceiveTick`
  (params (DeltaSeconds :type "Float (single-precision)"))
  (`self.K2_SetActorRotation` (`KismetMathLibrary.ComposeRotators` (`self.K2_GetActorRotation`) (struct :`Yaw` 10.0))))

(fn `GetSocketPosition`
  (params (Index :type Integer))
  (returns (NewParam :type "Vector Structure"))
  (return (`SceneComponent.GetSocketLocation` (`self.StaticMesh`) (`KismetStringLibrary.Conv_StringToName` (`KismetStringLibrary.Conv_IntToString` Index)))))

(fn `GetSocketTransform`
  (params (Index :type Integer))
  (returns (NewParam :type "Transform Structure"))
  (return (`SceneComponent.GetSocketTransform` (`self.StaticMesh`) (`KismetStringLibrary.Conv_StringToName` (`KismetStringLibrary.BuildString_Name` "" "pos_" (`KismetStringLibrary.Conv_StringToName` (`KismetStringLibrary.Conv_IntToString` Index)))) "RTS_World")))

(fn `UserConstructionScript`
  (set `self.BaseStaticMesh` (`self.StaticMesh`)))